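; DCPlayer is the player character, handling movement, look, jumping with a sound, interaction and the pause menu.
; Axis inputs feed the movement component and controller rotation, and BeginPlay stores the spawn transform.
; Interact runs a short Visibility line trace from the camera and calls EnableMessage on the blocking actor it hits.
; Pause creates a new DCPauseWidget on each press and adds it to the viewport without pausing the game here.
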(event `self.ReceiveBeginPlay`
  (set `self.SpawnTransform` (`self.GetTransform`)))

(event `InputAxis|MoveForwardBackward`
  (params (AxisValue :type "Float (single-precision)"))
  (`PawnMovementComponent.AddInputVector` (`self.CharacterMovement`) (* (`self.GetActorForwardVector`) AxisValue) false))

(event `InputAxis|MoveLeftRight`
  (params (AxisValue :type "Float (single-precision)"))
  (`PawnMovementComponent.AddInputVector` (`self.CharacterMovement`) (* (`self.GetActorRightVector`) AxisValue) false))

(event `InputAxis|LookUpDown`
  (params (AxisValue :type "Float (single-precision)"))
  (`self.AddControllerPitchInput` AxisValue))

(event `InputAxis|LookLeftRight`
  (params (AxisValue :type "Float (single-precision)"))
  (`self.AddControllerYawInput` AxisValue))

(event `InputAction|Jump`
  (params (Key :type "Key Structure"))
  (:`Pressed`
    (`self.Jump`)
    (`GameplayStatics.PlaySoundAtLocation` "/Game/Audio/jump_02.jump_02" (`SceneComponent.K2_GetComponentLocation` (`self.CapsuleComponent`)) (struct) 1.0 1.0 0.0 null null null))
  (:`Released`
    (`self.StopJumping`)))

(event `InputAction|Interact`
  (params (Key :type "Key Structure"))
  (bind _camera (`self.Camera`))
  (bind _returnvalue (`SceneComponent.K2_GetComponentLocation` _camera))
  (:`Pressed`
    (bind _outhit (`KismetSystemLibrary.LineTraceSingle` _returnvalue (+ _returnvalue (* (`SceneComponent.GetForwardVector` _camera) 300.0)) "TraceTypeQuery1"))
    (if (`GameplayStatics.BreakHitResult` _outhit)
      (message `/Game/Blueprints/DCInteractableInterface.Enable` (`.HitActor` (`GameplayStatics.BreakHitResult` _outhit))))))

(event `InputAction|Pause`
  (params (Key :type "Key Structure"))
  (:`Pressed`
    (bind _returnvalue (`|CreateWidget` "/Game/Widgets/DCPauseWidget.DCPauseWidget_C"))
    (bind _output_get (set `self.MenuRef` _returnvalue))
    (`UserWidget.AddToViewport` _output_get 0)))

(fn `UserConstructionScript`)